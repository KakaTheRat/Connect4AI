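; Game mode for Puissance 4 (Connect Four): two players alternately drop pawns into a six-row, seven-column board.
; NextTurn flips the player, spawns their pawn and hands it to the UserUI widget; PionPlacement positions it above a column.
; PlacePionInCase fills the lowest free cell via grid-to-world math, runs win checks, then always advances the turn.
; Row and column checks count non-consecutive pawns and only print wins; the diagonal check is unfinished.
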(event `self.ReceiveBeginPlay`
  (`self.InitBoard`)
  (`self.AddUI`)
  (`self.NextTurn`))

(event `RegisterPlayerController`
  (params (PC :type "/Game/PC_Puissance4 Object Reference"))
  (set `self.PlayerController` PC)
  (`self.SetCameraForPlayer`))

(event `SetCameraForPlayer`
  (bind _outactors (`GameplayStatics.GetAllActorsOfClass` "/Script/Engine.CameraActor"))
  (`PlayerController.SetViewTargetWithBlend` (`self.PlayerController`) (`|GetArrayItem` _outactors) 0.0 "VTBlend_Linear" 0.0 false))

(event `InitBoard`
  (bind _board (`self.Board`))
  (for _ (range 6)
    (`KismetArrayLibrary.Array_Add` _board (make `/Game/BoardLine` (`|MakeArray` 0 0 0 0 0 0 0))))
  (`KismetSystemLibrary.PrintString` (`KismetStringLibrary.Concat_StrStr` "Init with " (`KismetStringLibrary.Conv_IntToString` (`KismetArrayLibrary.Array_Length` _board)) " lines")))

(event `PlacePionInCase`
  (params (Case :type Integer) (Pion :type "Actor Object Reference"))
  (bind _playerturn (`self.PlayerTurn`))
  (for (_array_element _array_index) (`self.Board`)
    (if (== (`|GetArrayItem` (break `/Game/BoardLine` _array_element) Case) 0)
      (`self.PlacePion` (`self.PlayerTurn`) _array_index Case Pion)
      (break)))
  (`self.CheckWinHorizontal` _playerturn)
  (`self.CheckWinVertical` _playerturn)
  (`self.CheckWinDiagonal`)
  (`self.NextTurn`))

(event `PionPlacement`
  (params (Case :type Integer) (Pion :type "Actor Object Reference"))
  (bind _transform (`self.GetGoodLocation` 7 Case))
  (`self.K2_SetActorTransform` Pion (`KismetMathLibrary.MakeTransform` (- (.location _transform) (0.0 0.0 1000.0)) (.rotation _transform) (.scale _transform)) false false))

(event `AddUI`
  (bind _returnvalue (`|CreateWidget` "/Game/UserUI.UserUI_C" (`self.PlayerController`)))
  (bind _output_get (set `self.UserUI` _returnvalue))
  (`UserWidget.AddToViewport` _output_get 0))

(event `NextTurn`
  (`/Engine/EditorBlueprintResources/StandardMacros.FlipFlop`
    (:`A`
      (set `self.PlayerTurn` 1))
    (:`B`
      (set `self.PlayerTurn` 2)))
  (bind _pion (`self.GetRightPion` (`self.PlayerTurn`)))
  (`/Game/UserUI.NewTurn` (`self.UserUI`) _pion))

(fn `CheckWinDiagonal`
  (locals (PionInDiag :type Integer) (Win :type Boolean))
  (for _index (range 3)
    (for _index_2 (range 4)
      (set `local.PionInDiag` 0)
      (for _index_3 (range _index_2 (+ (+ _index_2 3) 1))
        (bind _output_line (break `/Game/BoardLine` (`|GetArrayItem` (`self.Board`) _index)))
        (if (== (`|GetArrayItem` _output_line _index_3) (`self.PlayerTurn`))
          (bind _result (`/Engine/EditorBlueprintResources/StandardMacros.IncrementInt` (`local.PionInDiag`))
            (:`  `
              (set `local.PionInDiag` _result)
              (`KismetSystemLibrary.PrintString` "+"))))))))

(fn `CheckWinHorizontal`
  (params (PlayerID :type Integer))
  (returns (`Win?` :type Boolean))
  (locals (PionInLine :type Integer) (IsWin :type Boolean))
  (for _array_element (`self.Board`)
    (set `local.PionInLine` 0)
    (for _array_element_2 (break `/Game/BoardLine` _array_element)
      (if (== _array_element_2 (`local.PlayerID`))
        (bind _result (`/Engine/EditorBlueprintResources/StandardMacros.IncrementInt` (`local.PionInLine`))
          (:`  `
            (bind _output_get (set `local.PionInLine` _result))
            (if (>= _output_get 4)
              (set `local.IsWin` true)
              (`KismetSystemLibrary.PrintString` (`KismetStringLibrary.Concat_StrStr` "Player " (`KismetStringLibrary.Conv_IntToString` (`self.PlayerTurn`)) " Win"))
              (return (`local.IsWin`))))))))
  (return (`local.IsWin`)))

(fn `CheckWinVertical`
  (params (PlayerID :type Integer))
  (returns (`Win?` :type Boolean))
  (locals (IsWin :type Boolean) (PionInColumn :type Integer))
  (for _index (range 7)
    (set `local.PionInColumn` 0)
    (for _array_element (`self.Board`)
      (if (== (`|GetArrayItem` (break `/Game/BoardLine` _array_element) _index) (`local.PlayerID`))
        (bind _result (`/Engine/EditorBlueprintResources/StandardMacros.IncrementInt` (`local.PionInColumn`))
          (:`  `
            (bind _output_get (set `local.PionInColumn` _result))
            (if (>= _output_get 4)
              (set `local.IsWin` true)
              (`KismetSystemLibrary.PrintString` (`KismetStringLibrary.Concat_StrStr` "Player " (`KismetStringLibrary.Conv_IntToString` (`self.PlayerTurn`)) " Win"))
              (return (`local.IsWin`))))))))
  (return (`local.IsWin`)))

(fn `GetGoodLocation`
  (params (Line :type Integer) (Case :type Integer))
  (returns (Transform :type "Transform Structure"))
  (return (`KismetMathLibrary.MakeTransform` (`KismetMathLibrary.MakeVector` (+ -125.0 (* Case 1940.0)) -4535.000022 (+ 950.0 (* Line 1610.0))) (struct :`Pitch` 90.0 :`Roll` 90.0))))

(fn `GetRightPion`
  (params (PlayerID :type Integer))
  (returns (Pion :type "Actor Object Reference"))
  (locals (GoodPion :type "Actor Object Reference"))
  (if (== PlayerID 1)
    (bind _returnvalue (`|SpawnActorFromClass` "/Game/P4/Player1Pion.Player1Pion_C" (`KismetMathLibrary.MakeTransform` (0.0 0.0 0.0)) "Undefined" "MultiplyWithRoot" null null))
    (set `local.GoodPion` _returnvalue)
    (else
      (bind _returnvalue_2 (`|SpawnActorFromClass` "/Game/P4/Player2Pion.Player2Pion_C" (`KismetMathLibrary.MakeTransform` (0.0 0.0 0.0)) "Undefined" "MultiplyWithRoot" null null))
      (set `local.GoodPion` _returnvalue_2)))
  (return (`local.GoodPion`)))

(fn `IsCaseEmpty`
  (params (Line :type Integer) (Case :type Integer))
  (returns (IsEmpy :type Boolean))
  (locals (Empty :type Boolean :default true))
  (bind _output_line (break `/Game/BoardLine` (`|GetArrayItem` (`self.Board`) Line)))
  (if (not (== (`|GetArrayItem` _output_line Case) 0))
    (set `local.Empty` false)
    (`KismetSystemLibrary.PrintString` "La case n'est pas vide"))
  (return (`local.Empty`)))

(fn `IsCaseFree`
  (params (Case :type Integer))
  (returns (IsFree :type Boolean))
  (locals (Free :type Boolean :default true))
  (bind _output_line (break `/Game/BoardLine` (`|GetArrayItem` (`self.Board`) 5)))
  (if (!= (`|GetArrayItem` _output_line Case) 0)
    (set `local.Free` false))
  (return (`local.Free`)))

(fn `PlacePion`
  (params (PlayerID :type Integer) (Line :type Integer) (Case :type Integer) (Pion :type "Actor Object Reference"))
  (returns (Placed :type Boolean))
  (locals (`Placé` :type Boolean :default true))
  (bind _line (`local.Line`))
  (bind _case (`local.Case`))
  (bind _isempy (`self.IsCaseEmpty` Line Case))
  (if _isempy
    (bind _transform (`self.GetGoodLocation` _line _case))
    (`self.K2_SetActorTransform` (`local.Pion`) _transform false false)
    (`self.UpdateBoardArray` (`local.PlayerID`) _line _case)
    (`KismetSystemLibrary.PrintString` "Pion placé")
    (else
      (set `local.Placé` false)
      (`KismetSystemLibrary.PrintString` "Pion non placé")))
  (return (`local.Placé`)))

(fn `UpdateBoardArray`
  (params (PlayerID :type Integer) (Line :type Integer) (Case :type Integer))
  (bind _output_line (break `/Game/BoardLine` (`|GetArrayItem` (`self.Board`) Line)))
  (`KismetArrayLibrary.Array_Set` _output_line Case PlayerID))

(fn `UserConstructionScript`)