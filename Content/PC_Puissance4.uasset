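; Player controller for the Puissance4 (Connect Four) game mode that registers itself with the game mode when play starts.
; On BeginPlay it casts the current game mode to GM_Puissance4, stores it, then calls RegisterPlayerController with itself.
; A failed cast only prints a message, and registration still runs on the unset reference.
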(event `self.ReceiveBeginPlay`
  (`self.GetGameMode`)
  (`self.RegisterPlayer`))

(event `GetGameMode`
  (bind _asgm_puissance_4 (cast `/Game/GM_Puissance4` (`GameplayStatics.GetGameMode`))
    (:`then`
      (set `self.GameMode` _asgm_puissance_4))
    (:`CastFailed`
      (`KismetSystemLibrary.PrintString` "Fail To Cast"))))

(event `RegisterPlayer`
  (`/Game/GM_Puissance4.RegisterPlayerController` (`self.GameMode`) self))

(fn `UserConstructionScript`)